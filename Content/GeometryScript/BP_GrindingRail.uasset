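; Procedural grinding rail built with Geometry Script as a generated mesh that follows a spline.
; On each rebuild it derives a temporary helper spline from the source spline, offset by Height with a corner radius.
; It samples that helper at a subdivision-based count, sweeps a circular profile along the frames to form the tube, then destroys the helper.
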(event Events|EventOnRebuildGeneratedMesh
  (params (TargetMesh :type Dynamic%20Mesh%20Object%20Reference))
  (Utilities|FlowControl|Sequence
    (:then_0
      (bind _returnvalue (Class|GeometryScriptLibraryPolyPathFunctions|CreateCirclePath2D "(X=0.000000,Y=0.000000)" (Variables|Default|GetRadius) (Variables|Default|GetRoudness)))
      (Variables|Default|SetBrush _returnvalue)
      (Utilities|IsValid 0
        (:Is%20Not%20Valid
          (bind _returnvalue_2 (Game|AddComponentbyClass "/Script/Engine.SplineComponent" false))
          (Variables|Default|SetHelperSpline _returnvalue_2))))
    (:then_1
      (Class|GeometryHelpers|CreateOffsettedSpline (Variables|Default|GetHelperSpline) (Variables|Default|GetSpline) (Math|Vector|MakeVector 0.0 0.0 (Variables|Default|GetHeight)) (Variables|Default|GetCorner%20Radius)))
    (:then_2
      (bind _frames (Class|GeometryScriptLibraryPolyPathFunctions|SampleSplinetoTransforms :Spline (Variables|Default|GetHelperSpline) :SamplingOptions (Utilities|Struct|MakeGeometryScriptSplineSamplingOptions (Math|Float|Truncate (|(((1+Subs)*(Points-1))+1) (Math|Conversions|ToFloat(Integer) (Variables|Default|GetSubdivision)) (Math|Conversions|ToFloat(Integer) (Spline|GetNumberOfSplinePoints (Variables|Default|GetHelperSpline))))) 1.0 "UniformDistance" "Local" "FullSpline" 0.0 1.0)))
      (Class|GeometryScriptLibraryMeshPrimitiveFunctions|AppendSweepPolygon :TargetMesh TargetMesh :PolygonVertices (Class|GeometryScriptLibraryPolyPathFunctions|ToArrayOfVector2D(GeometryScriptPolyPath) (Variables|Default|GetBrush)) :SweepPath _frames :Debug 0))
    (:then_3
      (Components|DestroyComponent (Variables|Default|GetHelperSpline)))))

(fn ConstructionScript)